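; Destructible cylinder actor built on a Geometry Collection that can fade its opacity on demand.
; The construction script registers the level's Anchor actor as the collection's initialization field and puts one dynamic material on both material slots.
; StartFade and EndFade play and reverse a timeline that lerps Opacity toward EndingFadeAmount.
; The first Chaos break event starts a delay, after which the actor destroys itself.
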(event `/Game/Blueprints/Iface/BPI_FadeInterface.StartFade`
  (bind (_direction _fadeamount) (`Timeline|FadeTimeline` :!label _label)
    (:`Update`
      (`MaterialInstanceDynamic.SetScalarParameterValue` (`self.DynamicMaterial`) "Opacity" (`KismetMathLibrary.Lerp` 1.0 (`self.EndingFadeAmount`) _fadeamount)))))

(event `/Game/Blueprints/Iface/BPI_FadeInterface.EndFade`
  (goto _label :!via `Reverse`))

(event `self.SM_Cylinder_GeometryCollection.OnChaosBreakEvent`
  (params (BreakEvent :type "ChaosBreakEvent Structure (by ref)"))
  (`/Engine/EditorBlueprintResources/StandardMacros.DoOnce` false
    (:`Completed`
      (`KismetSystemLibrary.Delay` 6.0)
      (`self.K2_DestroyActor`))))

(fn `UserConstructionScript`
  (bind _sm_cylinder_geometrycollection (`self.SM_Cylinder_GeometryCollection`))
  (bind _initializationfields (`GeometryCollectionComponent.InitializationFields` (`self.SM_Cylinder_GeometryCollection`)))
  (bind _output_get (set `self.MaterialToSet` (`PrimitiveComponent.GetMaterial` (`self.SM_Cylinder_GeometryCollection`) 0)))
  (`|ExecutionSequence`
    (:`then_0`
      (`KismetArrayLibrary.Array_Clear` _initializationfields)
      (bind _returnvalue (`GameplayStatics.GetActorOfClass` "/Game/Anchor.Anchor_C"))
      (`KismetArrayLibrary.Array_Add` _initializationfields _returnvalue))
    (:`then_1`
      (bind _returnvalue_2 (`PrimitiveComponent.CreateDynamicMaterialInstance` (`self.SM_Cylinder_GeometryCollection`) 0 _output_get "None"))
      (bind _output_get_2 (set `self.DynamicMaterial` _returnvalue_2))
      (`PrimitiveComponent.SetMaterial` _sm_cylinder_geometrycollection 0 _output_get_2)
      (`PrimitiveComponent.SetMaterial` _sm_cylinder_geometrycollection 1 _output_get_2))))