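; BP_CRS is a controller-driven character that caches references to the player, a BP_Poste, its spawn location and a BP_CrsControleur.
; Capsule overlaps are forwarded to its possessing BP_CrsControleur through IStouch.
; Tick switches between idle and crouched-walk animations based on nonzero X and Y velocity, each behind a DoOnce with no reset.
; StunCrs disables character movement for a few seconds, then restores it.
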(event `self.ReceiveBeginPlay`
  (bind _returnvalue (`GameplayStatics.GetActorOfClass` "/Game/TopDown/Blueprints/BP_TopDownCharacter.BP_TopDownCharacter_C"))
  (set `self.PlayerRef` _returnvalue)
  (bind _returnvalue_2 (`GameplayStatics.GetActorOfClass` "/Game/CRS/BP_Poste.BP_Poste_C"))
  (set `self.PosteRef` _returnvalue_2)
  (set `self.SpawnLocation` (`self.K2_GetActorLocation`))
  (bind _returnvalue_3 (`GameplayStatics.GetActorOfClass` "/Game/CRS/BP_CrsControleur.BP_CrsControleur_C"))
  (set `self.CrsControlleur` _returnvalue_3)
  (`SkeletalMeshComponent.PlayAnimation` (`self.Mesh`) "/Game/CRS/Anim/Standing_W_Briefcase_Idle.Standing_W_Briefcase_Idle" true))

(event `StartWalkAnim`)

(event `self.ReceiveTick`
  (params (DeltaSeconds :type "Float (single-precision)"))
  (bind _mesh (`self.Mesh`))
  (bind (_velocity_x _velocity_y) (`KismetMathLibrary.BreakVector` (`MovementComponent.Velocity` (`self.CharacterMovement`))))
  (if (and (or (> _velocity_x 0.0) (< _velocity_x 0.0)) (or (> _velocity_y 0.0) (< _velocity_y 0.0)))
    (`/Engine/EditorBlueprintResources/StandardMacros.DoOnce` false
      (:`Completed`
        (`SkeletalMeshComponent.PlayAnimation` _mesh "/Game/CRS/Anim/Crouched_Walking__1_.Crouched_Walking__1_" true)))
    (else
      (`/Engine/EditorBlueprintResources/StandardMacros.DoOnce` false
        (:`Completed`
          (`SkeletalMeshComponent.PlayAnimation` _mesh "/Game/CRS/Anim/Standing_W_Briefcase_Idle.Standing_W_Briefcase_Idle" true))))))

(event `self.CapsuleComponent.OnComponentBeginOverlap`
  (params (OverlappedComponent :type "PrimitiveComponent Object Reference") (OtherActor :type "Actor Object Reference") (OtherComp :type "PrimitiveComponent Object Reference") (OtherBodyIndex :type Integer) (bFromSweep :type Boolean) (SweepResult :type "HitResult Structure (by ref)"))
  (`KismetSystemLibrary.PrintString` "Hello")
  (bind _asbp_crs_controleur (cast `/Game/CRS/BP_CrsControleur` (`self.GetController`)))
  (`/Game/CRS/BP_CrsControleur.IStouch` _asbp_crs_controleur OtherActor self))

(event `StunCrs`
  (`ActorComponent.SetActive` (`self.CharacterMovement`) false false)
  (`KismetSystemLibrary.Delay` 3.0)
  (`ActorComponent.SetActive` (`self.CharacterMovement`) true false))

(fn `UserConstructionScript`)