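; AI controller for the CRS enemy, which takes gnomes from the top-down player and carries them to the Poste.
; On perceiving the player, it chases the last gnome in AllGnomes.
; Touch events drive the cycle: destroy the gnome, show a carried mini-gnome, disable sight, deliver, then return to spawn.
; Sight resumes at spawn if gnomes remain, otherwise a looping timer polls until the array refills.
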(event `self.ReceiveBeginPlay`
  (bind _returnvalue (`GameplayStatics.GetActorOfClass` "/Game/CRS/BP_CRS.BP_CRS_C"))
  (set `self.CrsRef` _returnvalue)
  (bind _returnvalue_2 (`GameplayStatics.GetActorOfClass` "/Game/TopDown/Blueprints/BP_TopDownCharacter.BP_TopDownCharacter_C"))
  (set `self.PlayerRef` _returnvalue_2)
  (bind _returnvalue_3 (`GameplayStatics.GetActorOfClass` "/Game/CRS/BP_Poste.BP_Poste_C"))
  (set `self.PosteRef` _returnvalue_3))

(event `self.AIPerception.OnPerceptionUpdated`
  (params (UpdatedActors :type "Array of Actor Object Reference (by ref)"))
  (bind _playerref (`self.PlayerRef`))
  (bind _playerref_2 (`self.PlayerRef`))
  (bind _allgnomes (`/Game/TopDown/Blueprints/BP_TopDownCharacter.AllGnomes` _playerref))
  (for _array_element UpdatedActors
    (bind _asbp_top_down_character (cast `/Game/TopDown/Blueprints/BP_TopDownCharacter` _array_element)
      (:`then`
        (`KismetSystemLibrary.PrintString` "Valid")
        (if (== _asbp_top_down_character (`self.PlayerRef`))
          (`/Engine/EditorBlueprintResources/StandardMacros.IsValid` _playerref
            (:`Is Valid`
              (if (`KismetArrayLibrary.Array_IsEmpty` _allgnomes)
                (`KismetSystemLibrary.PrintString` "not valid2")
                (set `/Game/TopDown/Blueprints/BP_TopDownCharacter.LastGnome` _playerref_2 _playerref_2)
                (else
                  (bind _output_get (set `self.Target` (`|GetArrayItem` _allgnomes (`KismetArrayLibrary.Array_LastIndex` _allgnomes))))
                  (`AITask_MoveTo.AIMoveTo` null (0.0 0.0 0.0) _output_get -1.0 "Disable" "Enable" true true true))))
            (:`Is Not Valid`
              (`KismetSystemLibrary.PrintString` "not valid1")))))
      (:`CastFailed`
        (`KismetSystemLibrary.PrintString` "not vali0")))))

(event `IStouch`
  (params (Actor :type "Actor Object Reference"))
  (bind _playerref (`self.PlayerRef`))
  (bind _target (`self.Target`))
  (bind _allgnomes (`/Game/TopDown/Blueprints/BP_TopDownCharacter.AllGnomes` (`self.PlayerRef`)))
  (if (== Actor _target)
    (`self.K2_DestroyActor` _target)
    (`KismetArrayLibrary.Array_Remove` _allgnomes (`KismetArrayLibrary.Array_LastIndex` _allgnomes))
    (`KismetSystemLibrary.Delay` 1.0)
    (`SceneComponent.SetVisibility` (`/Game/CRS/BP_CRS.Petit_Gnome` (`self.CrsRef`)) true false)
    (`AIPerceptionComponent.SetSenseEnabled` (`self.AIPerception`) "/Script/AIModule.AISense_Sight" false)
    (`AITask_MoveTo.AIMoveTo` null (0.0 0.0 0.0) (`self.PosteRef`) -1.0 "Disable" "Enable" true true true)
    (elif (== Actor (`self.PosteRef`))
      (`SceneComponent.SetVisibility` (`/Game/CRS/BP_CRS.Petit_Gnome` (`self.CrsRef`)) false false)
      (`AITask_MoveTo.AIMoveTo` null (`/Game/CRS/BP_CRS.SpawnLocation` (`self.CrsRef`)) null -1.0 "Disable" "Enable" true true true
        (:`OnMoveFinished`
          (if (`KismetArrayLibrary.Array_IsEmpty` (`/Game/TopDown/Blueprints/BP_TopDownCharacter.AllGnomes` (`self.PlayerRef`)))
            (set `/Game/TopDown/Blueprints/BP_TopDownCharacter.LastGnome` _playerref _playerref)
            (`KismetSystemLibrary.K2_SetTimerDelegate` (delegate `CustomEvent`) 0.1 true)
            (else
              (`AIPerceptionComponent.SetSenseEnabled` (`self.AIPerception`) "/Script/AIModule.AISense_Sight" true))))))))

(event `CustomEvent`
  (if (`KismetArrayLibrary.Array_IsEmpty` (`/Game/TopDown/Blueprints/BP_TopDownCharacter.AllGnomes` (`self.PlayerRef`)))
    (`KismetSystemLibrary.PrintString` "tableau vide")
    (else
      (`AIPerceptionComponent.SetSenseEnabled` (`self.AIPerception`) "/Script/AIModule.AISense_Sight" true))))

(fn `UserConstructionScript`)