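; BP_Poste is a mesh actor that can fade its Cube's opacity out and back on request.
; The construction script replaces each Cube material with a dynamic instance stored in DynamicMaterial.
; StartFade plays a timeline that lerps every instance's Opacity parameter from opaque toward EndingFadeAmount, and EndFade reverses it.
; A BP_CRS spawn at the Arrow's transform exists but is unconnected, so never runs.
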(event `/Game/Blueprints/Iface/BPI_FadeInterface.StartFade`
  (bind (_direction _fadeamount) (`Timeline|Timeline` :!label _label)
    (:`Update`
      (for _array_element (`self.Dynamic Material`)
        (`MaterialInstanceDynamic.SetScalarParameterValue` _array_element "Opacity" (`KismetMathLibrary.Lerp` 1.0 (`self.EndingFadeAmount`) _fadeamount))))))

(event `/Game/Blueprints/Iface/BPI_FadeInterface.EndFade`
  (goto _label :!via `Reverse`))

(fn `UserConstructionScript`
  (bind _cube (`self.Cube`))
  (`KismetArrayLibrary.Array_Clear` (`self.Dynamic Material`))
  (for (_array_element _array_index) (`MeshComponent.GetMaterials` _cube)
    (bind _returnvalue (`PrimitiveComponent.CreateDynamicMaterialInstance` _cube _array_index _array_element "None"))
    (`KismetArrayLibrary.Array_Add` (`self.Dynamic Material`) _returnvalue)
    (`PrimitiveComponent.SetMaterial` _cube _array_index _returnvalue)))