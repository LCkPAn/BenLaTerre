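; BP_Gnome is an AI-controlled gnome that walks toward a Target actor with a waddling motion.
; On BeginPlay, a looping timer repeatedly calls FollowGnogme, which issues SimpleMoveToActor through the gnome's AI controller.
; The Dodeline timeline also starts there, using its WalkLikeAGnome track to drive the mesh's relative pitch, faking a gnome walk by rotation.
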(event `self.ReceiveBeginPlay`
  (bind _mesh (`self.Mesh`))
  (bind (_relativerotation_roll _relativerotation_pitch _relativerotation_yaw) (`KismetMathLibrary.BreakRotator` (`SceneComponent.RelativeRotation` _mesh)))
  (bind _returnvalue (`KismetSystemLibrary.K2_SetTimerDelegate` (delegate `FollowGnogme`) 0.1 true))
  (set `self.TimerRef` _returnvalue)
  (bind (_direction _walklikeagnome) (`Timeline|Dodeline`)
    (:`Update`
      (`SceneComponent.K2_SetRelativeRotation` _mesh (`KismetMathLibrary.MakeRotator` _relativerotation_roll (`KismetMathLibrary.Lerp` 0.0 40.0 _walklikeagnome) _relativerotation_yaw) false false))))

(event `FollowGnogme`
  (`AIBlueprintHelperLibrary.SimpleMoveToActor` (`AIBlueprintHelperLibrary.GetAIController` self) (`self.Target`)))

(fn `UserConstructionScript`)