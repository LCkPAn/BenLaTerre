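; BP_ThrowGnogne is a thrown gnome actor that reacts to whatever its collision component hits.
; On BeginPlay it rotates that component and caches the BP_CRS actor, which it stuns on impact before destroying itself.
; The first hit on a BPI_FadeInterface actor briefly spawns Fs_MasterFieldCopy at the impact point, apparently a destruction field, then removes both.
; Other hits destroy the gnome after a delay; non-CRS hits also print debug text.
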(event `self.ReceiveBeginPlay`
  (bind _collision (`self.Collision`))
  (`SceneComponent.K2_SetRelativeRotation` _collision (`KismetMathLibrary.RotatorFromAxisAndAngle` (`SceneComponent.GetRightVector` _collision) 90.0) false false)
  (bind _returnvalue (`GameplayStatics.GetActorOfClass` "/Game/CRS/BP_CRS.BP_CRS_C"))
  (set `self.CrsRef` _returnvalue))

(event `self.Collision.OnComponentHit`
  (params (HitComponent :type "PrimitiveComponent Object Reference") (OtherActor :type "Actor Object Reference") (OtherComp :type "PrimitiveComponent Object Reference") (NormalImpulse :type "Vector Structure") (Hit :type "HitResult Structure (by ref)"))
  (if (== OtherActor (`self.CrsRef`))
    (`/Game/CRS/BP_CRS.StunCrs` (`self.CrsRef`))
    (`KismetSystemLibrary.Delay` 1.0)
    (`self.K2_DestroyActor`)
    (else
      (`KismetSystemLibrary.PrintString` "Hello")
      (if (`KismetSystemLibrary.DoesImplementInterface` OtherActor "/Game/Blueprints/Iface/BPI_FadeInterface.BPI_FadeInterface_C")
        (`/Engine/EditorBlueprintResources/StandardMacros.DoOnce` false
          (:`Completed`
            (bind _returnvalue (`|SpawnActorFromClass` "/Game/Fs_MasterFieldCopy.Fs_MasterFieldCopy_C" (`KismetMathLibrary.MakeTransform` (`.Location` (`GameplayStatics.BreakHitResult` Hit))) "Undefined" "OverrideRootScale" null null))
            (`KismetSystemLibrary.Delay` 0.3)
            (`self.K2_DestroyActor` _returnvalue)
            (`self.K2_DestroyActor`)))
        (else
          (`KismetSystemLibrary.Delay` 3.0)
          (`self.K2_DestroyActor`))))))

(fn `UserConstructionScript`)